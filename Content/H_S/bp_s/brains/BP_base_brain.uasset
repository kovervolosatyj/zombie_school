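; Base brain Blueprint that tracks rot and a timed lifespan, with empty Combat and Movement functions.
; While Empty, Tick raises CurrentRot up to MaxRot, and resetonhit subtracts from it within the same clamp.
; Separately, BeginPlay starts a one-minute timer that refresh clears and restarts.
; An onbrainexpired event broadcasts OnBrainExp, though the timer's bound event is not shown.
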(event Custom|on%20brain%20expired
  (Default|CallOnBrainExp))

(event Custom|rotting
  (bind _returnvalue (Utilities|Time|SetTimerbyEvent (EventDispatchers|CreateEvent :!event Custom|on%20brain%20expired) 6e+01))
  (Variables|Default|Setprime_handle _returnvalue))

(event Custom|refresh
  (Utilities|Time|ClearandInvalidateTimerbyHandle (Variables|Default|Getprime_handle))
  (CallFunction|Rotting))

(event Custom|reset%20on%20hit
  (params (minus%20value :type Float%20%28double-precision%29))
  (Variables|Default|Setcurrent_rot (Math|Float|Clamp(Float) (- (Variables|Default|Getcurrent_rot) minus%20value) 0.0 (Variables|Default|Getmax%20rot))))

(event EventBeginPlay
  (CallFunction|Rotting))

(event EventTick
  (params (DeltaSeconds :type Float%20%28single-precision%29))
  (if (Variables|Default|Getempty)
    (Variables|Default|Setcurrent_rot (Math|Float|Clamp(Float) (+ (* DeltaSeconds 1.66) (Variables|Default|Getcurrent_rot)) 0.0 (Variables|Default|Getmax%20rot)))))

(fn Combat)

(fn Movement)