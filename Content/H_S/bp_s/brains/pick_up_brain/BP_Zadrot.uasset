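; BP_Zadrot is a brain pickup actor that grants the Zadrot brain to a BP_H_S character when it overlaps the pickup's box.
; If the primary slot is default, it sets the Zadrot flag, clears the Zadira and Stacy flags, invalidates the Expired and Sup timers, and calls ZadrotPickUp and ZadrotEvent.
; Otherwise, a default secondary slot receives only ZadrotPickUp.
; The actor destroys itself after either successful pickup.
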(event OnComponentBeginOverlap(Box)
  (params (OverlappedComponent :type Primitive%20Component%20Object%20Reference) (OtherActor :type Actor%20Object%20Reference) (OtherComp :type Primitive%20Component%20Object%20Reference) (OtherBodyIndex :type Integer) (bFromSweep :type Boolean) (SweepResult :type Hit%20Result%20Structure%20%28by%20ref%29))
  (bind _asbp_h_s (Utilities|Casting|CastToBP_H_S OtherActor))
  (if (Variables|/Game/H_S/bp_s/brains/BP_base_brain.BP_base_brain_C|Getisdefault (Variables|/Game/H_S/BP_H_S.BP_H_S_C|GetSlot_primary _asbp_h_s))
    (Variables|/Game/H_S/BP_H_S.BP_H_S_C|SetZadrot _asbp_h_s true)
    (Variables|/Game/H_S/BP_H_S.BP_H_S_C|SetZadira _asbp_h_s false)
    (Variables|/Game/H_S/BP_H_S.BP_H_S_C|SetStacy _asbp_h_s false)
    (Default|ZadrotPickUp _asbp_h_s)
    (Utilities|Time|ClearandInvalidateTimerbyHandle (Variables|/Game/H_S/BP_H_S.BP_H_S_C|Getexpired_handle _asbp_h_s))
    (Utilities|Time|ClearandInvalidateTimerbyHandle (Variables|/Game/H_S/BP_H_S.BP_H_S_C|Getsup_handle _asbp_h_s))
    (Default|ZadrotEvent _asbp_h_s)
    (Actor|DestroyActor :!label _label)
    (elif (Variables|/Game/H_S/bp_s/brains/BP_base_brain.BP_base_brain_C|Getisdefault (Variables|/Game/H_S/BP_H_S.BP_H_S_C|GetSlot_secondary _asbp_h_s))
      (Default|ZadrotPickUp _asbp_h_s)
      (goto _label))))

(event EventBeginPlay)

(event Collision|EventActorBeginOverlap
  (params (OtherActor :type Actor%20Object%20Reference)))

(event EventTick
  (params (DeltaSeconds :type Float%20%28single-precision%29)))

(fn ConstructionScript)