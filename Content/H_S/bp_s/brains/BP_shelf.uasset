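; BP_shelf is a shelf trigger that randomly yields a healing or damaging effect when a BP_H_S actor enters its Box.
; On each overlap, a coin flip spawns either PR_heal or PR_damage at the shelf's transform.
; Both outcomes play a bottle sound at the overlapping actor's location, and the heal outcome adds a heal sound after a short delay.
; No guard limits it to a single use.
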(event OnComponentBeginOverlap(Box)
  (params (OverlappedComponent :type Primitive%20Component%20Object%20Reference) (OtherActor :type Actor%20Object%20Reference) (OtherComp :type Primitive%20Component%20Object%20Reference) (OtherBodyIndex :type Integer) (bFromSweep :type Boolean) (SweepResult :type Hit%20Result%20Structure%20%28by%20ref%29))
  (bind _asbp_h_s (Utilities|Casting|CastToBP_H_S OtherActor))
  (if (Math|Random|RandomBool)
    (Game|SpawnActorfromClass "/Game/H_S/proj/PR_heal.PR_heal_C" (Transformation|GetActorTransform) "Undefined" "MultiplyWithRoot" 0 0)
    (Audio|PlaySoundatLocation "/Game/Sounds/bottle_Cue.bottle_Cue" (Transformation|GetActorLocation _asbp_h_s) "0, 0, 0" 1.0 1.0 0.0 0 0 0 0)
    (Utilities|FlowControl|Delay 0.2)
    (Audio|PlaySoundatLocation "/Game/Sounds/Heal_Cue.Heal_Cue" (Transformation|GetActorLocation _asbp_h_s) "0, 0, 0" 1.0 1.0 0.0 0 0 0 0)
    (else
      (Game|SpawnActorfromClass "/Game/H_S/proj/PR_damage.PR_damage_C" (Transformation|GetActorTransform) "Undefined" "MultiplyWithRoot" 0 0)
      (Audio|PlaySoundatLocation "/Game/Sounds/bottle_Cue.bottle_Cue" (Transformation|GetActorLocation _asbp_h_s) "0, 0, 0" 1.0 1.0 0.0 0 0 0 0))))

(event EventBeginPlay)

(event Collision|EventActorBeginOverlap
  (params (OtherActor :type Actor%20Object%20Reference)))

(event EventTick
  (params (DeltaSeconds :type Float%20%28single-precision%29)))

(fn ConstructionScript)