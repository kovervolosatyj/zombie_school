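; BP_shelf_b is a shelf actor that spawns a random character when a BP_H_S actor overlaps its Box.
; The overlap picks BP_Stacy, BP_Zadira or BP_Zadrot and spawns it 200 units along negative world X from the shelf.
; Each choice has its own DoOnce gate, and all three gates reset after a shared 1.5-second Delay.
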(event OnComponentBeginOverlap(Box)
  (params (OverlappedComponent :type Primitive%20Component%20Object%20Reference) (OtherActor :type Actor%20Object%20Reference) (OtherComp :type Primitive%20Component%20Object%20Reference) (OtherBodyIndex :type Integer) (bFromSweep :type Boolean) (SweepResult :type Hit%20Result%20Structure%20%28by%20ref%29))
  (bind _returnvalue (Transformation|GetActorLocation))
  (bind _returnvalue_2 (+ _returnvalue "-200.000000,0.000000,0.000000"))
  (Utilities|Casting|CastToBP_H_S OtherActor)
  (switch int (Math|Random|RandomIntegerinRange 0 2)
    (:0
      (Utilities|FlowControl|DoOnce false :!label _label
        (:Completed
          (Game|SpawnActorfromClass "/Game/H_S/bp_s/brains/pick_up_brain/BP_Stacy.BP_Stacy_C" (Math|Transform|MakeTransform _returnvalue_2 "0, 0, 0" "1.000000,1.000000,1.000000") "Undefined" "MultiplyWithRoot" 0 0))))
    (:1
      (Utilities|FlowControl|DoOnce false :!label _label_2
        (:Completed
          (Game|SpawnActorfromClass "/Game/H_S/bp_s/brains/pick_up_brain/BP_Zadira.BP_Zadira_C" (Math|Transform|MakeTransform _returnvalue_2 "0, 0, 0" "1.000000,1.000000,1.000000") "Undefined" "MultiplyWithRoot" 0 0))))
    (:2
      (Utilities|FlowControl|DoOnce false :!label _label_3
        (:Completed
          (Game|SpawnActorfromClass "/Game/H_S/bp_s/brains/pick_up_brain/BP_Zadrot.BP_Zadrot_C" (Math|Transform|MakeTransform _returnvalue_2 "0, 0, 0" "1.000000,1.000000,1.000000") "Undefined" "MultiplyWithRoot" 0 0)))))
  (Utilities|FlowControl|Delay 1.5)
  (Utilities|FlowControl|Sequence
    (:then_0
      (goto _label Reset))
    (:then_1
      (goto _label_2 Reset))
    (:then_2
      (goto _label_3 Reset))))

(event EventBeginPlay)

(event Collision|EventActorBeginOverlap
  (params (OtherActor :type Actor%20Object%20Reference)))

(event EventTick
  (params (DeltaSeconds :type Float%20%28single-precision%29)))

(fn ConstructionScript)